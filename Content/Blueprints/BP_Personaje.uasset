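; BP_Personaje is a character Blueprint that moves itself every frame and can speed up when attacked.
; Tick adds the Velocidad vector as a local offset, without sweep or delta-time scaling.
; BeginPlay sets a non-looping timer that checks MeAtacan once and, if true, doubles Velocidad after a short delay.
; The functions VelocidadDeMovimiento and EstoySiendoAtacado act as setters for speed and attack state.
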(event Custom|Está%20Siendo%20Atacado
  ;[1 1 1] Cada 2 segundos el personaje comprueba si está ciendo atacado, si es atacado va a multiplicar su velocidad por 2 y setea su nueva velocidad, esto lo hace una vez, por lo cual no se deja tilda el looping
  (if (Variables|Default|GetMeAtacan)
    (Utilities|FlowControl|Delay 1.0)
    (Variables|Default|SetVelocidad (* (Variables|Default|GetVelocidad) 2))))

(event EventBeginPlay
  ;[1 1 1] Cada 2 segundos el personaje comprueba si está ciendo atacado, si es atacado va a multiplicar su velocidad por 2 y setea su nueva velocidad, esto lo hace una vez, por lo cual no se deja tilda el looping
  (Utilities|Time|SetTimerbyEvent (delegate Custom|Está%20Siendo%20Atacado) 2.0))

(event EventTick
  (params (DeltaSeconds :type Float%20%28single-precision%29))
  ;[1 1 1] Movimiento con nua velocidad editable
  (Transformation|AddActorLocalOffset (Variables|Default|GetVelocidad) false false))

(fn ConstructionScript)

(fn VelocidadDeMovimiento
  (params (Velocidad :type Vector))
  (Variables|Default|SetVelocidad Velocidad))

(fn EstoySiendoAtacado
  (params (MeAtacan :type Boolean))
  (Variables|Default|SetMeAtacan MeAtacan))